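; BP_Actor is an actor that exercises basic Blueprint flow control and prints the results on BeginPlay.
; A Sequence node prints the GameLevel variable before and after setting it, checks it against a threshold to print a confirmation, then runs a counted loop that prints each index and a completion message.
; Overlap, Tick and the construction script are empty.
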(event EventBeginPlay
  (Utilities|FlowControl|Sequence
    (:then_0
      (Development|PrintString (Utilities|String|ToString(Integer) (Variables|Default|GetGameLevel)))
      (bind _output_get (Variables|Default|SetGameLevel 10))
      (Development|PrintString (Utilities|String|ToString(Integer) _output_get)))
    (:then_1
      (if (>= (Variables|Default|GetGameLevel) 10)
        (Development|PrintString "Good!")))
    (:then_2
      (for _index (range 0 9)
        (Development|PrintString (Utilities|String|ToString(Integer) _index)))
      (Development|PrintString "Loop End!"))))

(event Collision|EventActorBeginOverlap
  (params (OtherActor :type Actor%20Object%20Reference)))

(event EventTick
  (params (DeltaSeconds :type Float%20%28single-precision%29)))

(fn ConstructionScript)